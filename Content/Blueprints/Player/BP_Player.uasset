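; Player Blueprint that handles pausing and the game over screen.
; The Pause input calls OnPause, where a FlipFlop alternates between pausing with a newly created PauseMenu_UI and unpausing by removing all top-level instances of that widget.
; DisplayGameOver pauses the game and shows GameOver_UI.
; Both screens show the mouse cursor, which is hidden again on unpause.
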(event Custom|OnPause
  (bind _returnvalue (Game|GetPlayerController 0))
  (Utilities|FlowControl|FlipFlop
    (:A
      ;[1 1 1] Pause Game
      (Game|SetGamePaused true)
      (Utilities|IsValid (Variables|Default|GetPauseMenu)
        (:Is%20Valid
          _)
        (:Is%20Not%20Valid
          _))
      (bind _returnvalue_2 (UserInterface|CreateWidget "/Game/UI/PauseMenu_UI.PauseMenu_UI_C" _returnvalue))
      (Variables|Default|SetPauseMenu _returnvalue_2)
      (UserInterface|Viewport|AddtoViewport (Variables|Default|GetPauseMenu) 0)
      (Variables|/Script/Engine.PlayerController|SetbShowMouseCursor _returnvalue true))
    (:B
      ;[1 1 1] Unpause Game
      (Game|SetGamePaused false)
      (bind _foundwidgets (Widget|GetAllWidgetsOfClass "/Game/UI/PauseMenu_UI.PauseMenu_UI_C" true))
      (Widget|RemovefromParent _foundwidgets)
      (Variables|/Script/Engine.PlayerController|SetbShowMouseCursor (Game|GetPlayerController 0) false))))

(event EventBeginPlay)

(event Collision|EventActorBeginOverlap
  (params (OtherActor :type Actor%20Object%20Reference)))

(event EventTick
  (params (DeltaSeconds :type Float%20%28single-precision%29)))

(event EventDisplayGameOver
  (bind _returnvalue (Game|GetPlayerController 0))
  ;[1 1 1] Game Over
  (Game|SetGamePaused true)
  (bind _returnvalue_2 (UserInterface|CreateWidget "/Game/UI/GameOver_UI.GameOver_UI_C" _returnvalue))
  (bind _output_get (Variables|Default|SetNewVar_0 _returnvalue_2))
  (UserInterface|Viewport|AddtoViewport _output_get 0)
  (Variables|/Script/Engine.PlayerController|SetbShowMouseCursor _returnvalue true))

(event Input|ActionEvents|InputActionPause
  (params (Key :type Key%20Structure :default "None"))
  (:Pressed
    (CallFunction|OnPause)))

(fn ConstructionScript)