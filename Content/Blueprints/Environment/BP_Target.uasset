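; BP_Target is a destructible target actor that adds itself to the FiftyMinInsideGameMode target counter on BeginPlay.
; Each BP_Flare hit destroys the flare and advances DamageIndex, recoloring the mesh through a dynamic material instance.
; A hit at damage index 2 decrements the counter and destroys the target.
; UpdateCustomDepth toggles the mesh's custom depth rendering and re-applies SM_Target in both branches.
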(event OnComponentHit(StaticMesh)
  (params (HitComponent :type Primitive%20Component%20Object%20Reference) (OtherActor :type Actor%20Object%20Reference) (OtherComp :type Primitive%20Component%20Object%20Reference) (NormalImpulse :type Vector :default "0, 0, 0") (Hit :type Hit%20Result%20Structure%20%28by%20ref%29))
  (bind _damageindex (Variables|Default|GetDamageIndex))
  ;[1 1 1] Increase Target's Hit Counter
  (bind _asbp_flare (Utilities|Casting|CastToBP_Flare OtherActor))
  (Actor|DestroyActor _asbp_flare)
  (if (== _damageindex 2)
    (Class|FiftyMinInsideGameMode|SetTargetCounter (Variables|Default|GetGameMode) -1)
    (Actor|DestroyActor)
    (else
      (Math|Integer|IncrementInt _damageindex
        (:%20%20
          ;[1 1 1] Set Target Material
          (bind _returnvalue (Rendering|Material|CreateDynamicMaterialInstance "/Engine/VREditor/LaserPointer/LaserPointerMaterial.LaserPointerMaterial" "None" :!class /Script/Engine.KismetMaterialLibrary))
          (bind _output_get (Variables|Default|SetMatInstance _returnvalue))
          (Rendering|Material|SetVectorParameterValue _output_get "LaserColor" (Math|Conversions|ToLinearColor(Vector) (Utilities|Array|Get(acopy) (Variables|Default|GetColors) (Variables|Default|GetDamageIndex))) :!class /Script/Engine.MaterialInstanceDynamic)
          (Rendering|Material|SetMaterial (Variables|Default|GetStaticMesh) 0 _output_get))))))

(event Custom|UpdateCustomDepth
  (bind _staticmesh (Variables|Default|GetStaticMesh))
  ;[1 1 1] Update target's custom depth
  (if (Variables|/Script/Engine.PrimitiveComponent|GetbRenderCustomDepth _staticmesh)
    (Rendering|SetRenderCustomDepth _staticmesh false)
    (Components|StaticMesh|SetStaticMesh _staticmesh "/Game/Meshes/SM_Target.SM_Target")
    (else
      (Rendering|SetRenderCustomDepth _staticmesh true)
      (Components|StaticMesh|SetStaticMesh _staticmesh "/Game/Meshes/SM_Target.SM_Target"))))

(event EventBeginPlay
  ;[1 1 1] Init Level
  (bind _asfifty_min_inside_game_mode (Utilities|Casting|CastToFiftyMinInsideGameMode (Game|GetGameMode)))
  (Variables|Default|SetGameMode _asfifty_min_inside_game_mode)
  (Class|FiftyMinInsideGameMode|SetTargetCounter _asfifty_min_inside_game_mode 1)
  ;[1 1 1] Set Target Material
  (bind _returnvalue (Rendering|Material|CreateDynamicMaterialInstance "/Engine/VREditor/LaserPointer/LaserPointerMaterial.LaserPointerMaterial" "None" :!class /Script/Engine.KismetMaterialLibrary))
  (bind _output_get (Variables|Default|SetMatInstance _returnvalue))
  (Rendering|Material|SetVectorParameterValue _output_get "LaserColor" (Math|Conversions|ToLinearColor(Vector) (Utilities|Array|Get(acopy) (Variables|Default|GetColors) (Variables|Default|GetDamageIndex))) :!class /Script/Engine.MaterialInstanceDynamic)
  (Rendering|Material|SetMaterial (Variables|Default|GetStaticMesh) 0 _output_get))

(fn ConstructionScript)