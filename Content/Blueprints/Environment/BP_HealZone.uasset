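; BP_HealZone is a healing area that restores the player pawn's health while it stands inside a box volume.
; Box overlap events set an IsOverlapping flag when a FiftyMinInsidePawn enters or leaves.
; On Tick, while the flag is set, it calls UpdateHealth on the player pawn cached at BeginPlay with a frame-rate-independent amount per second.
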(event OnComponentBeginOverlap(Box)
  (params (OverlappedComponent :type Primitive%20Component%20Object%20Reference) (OtherActor :type Actor%20Object%20Reference) (OtherComp :type Primitive%20Component%20Object%20Reference) (OtherBodyIndex :type Integer) (bFromSweep :type Boolean) (SweepResult :type Hit%20Result%20Structure%20%28by%20ref%29))
  (Utilities|Casting|CastToFiftyMinInsidePawn OtherActor)
  (Variables|Default|SetIsOverlapping true))

(event OnComponentEndOverlap(Box)
  (params (OverlappedComponent :type Primitive%20Component%20Object%20Reference) (OtherActor :type Actor%20Object%20Reference) (OtherComp :type Primitive%20Component%20Object%20Reference) (OtherBodyIndex :type Integer))
  (Utilities|Casting|CastToFiftyMinInsidePawn OtherActor)
  (Variables|Default|SetIsOverlapping false))

(event EventBeginPlay
  (bind _asfifty_min_inside_pawn (Utilities|Casting|CastToFiftyMinInsidePawn (Game|Player|GetPlayerPawn 0)))
  (Variables|Default|SetPlayerPawn _asfifty_min_inside_pawn))

(event EventTick
  (params (DeltaSeconds :type Float%20%28single-precision%29))
  (if (Variables|Default|GetIsOverlapping)
    (Class|FiftyMinInsidePawn|UpdateHealth (Variables|Default|GetPlayerPawn) (* DeltaSeconds 5.0))))

(fn ConstructionScript
  (|CallParentFunction))